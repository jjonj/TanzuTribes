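; RTS camera actor that pans over terrain and zooms on a spring arm, with projection settings applied in the construction script.
; Each tick, axis input becomes a yaw-relative pan, scaled by a zoom-based curve and doubled with Left Shift.
; A downward trace holds the actor above the ground, smoothing only height changes.
; ZoomIn and ZoomOut set a clamped, curve-scaled arm length target that Tick interpolates toward.
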(event Custom|ZoomIn
  (bind _cameraboom (Variables|Default|GetCameraBoom))
  (bind _targetarmlength (Variables|/Script/Engine.SpringArmComponent|GetTargetArmLength _cameraboom))
  ;[1 1 1] Zoom Events
  (Variables|RTSCamera|SetCameraBoomLength (Math|Float|Clamp(Float) (- _targetarmlength (* (Math|Curves|GetFloatValue (Variables|RTSCamera|GetZoomRateCurve) _targetarmlength) (Variables|RTSCamera|GetBaseZoomRate))) (Variables|RTSCamera|GetMinZoom) (Variables|RTSCamera|GetMaxZoom))))

(event Custom|ZoomOut
  (bind _cameraboom (Variables|Default|GetCameraBoom))
  (bind _targetarmlength (Variables|/Script/Engine.SpringArmComponent|GetTargetArmLength _cameraboom))
  ;[1 1 1] Zoom Events
  (Variables|RTSCamera|SetCameraBoomLength (Math|Float|Clamp(Float) (+ _targetarmlength (* (Math|Curves|GetFloatValue (Variables|RTSCamera|GetZoomRateCurve) _targetarmlength) (Variables|RTSCamera|GetBaseZoomRate))) (Variables|RTSCamera|GetMinZoom) (Variables|RTSCamera|GetMaxZoom))))

(event EventTick
  (params (DeltaSeconds :type Float%20%28single-precision%29))
  (bind _mainroot (Variables|Default|GetMainRoot))
  (bind _cameramovementspeed (Variables|RTSCamera|GetCameraMovementSpeed))
  (bind _cameraboom (Variables|Default|GetCameraBoom))
  ;[1 1 1] Zoom Interp
  (Variables|/Script/Engine.SpringArmComponent|SetTargetArmLength _cameraboom (Math|Interpolation|FInterpTo (Variables|/Script/Engine.SpringArmComponent|GetTargetArmLength _cameraboom) (Variables|RTSCamera|GetCameraBoomLength) DeltaSeconds (Variables|RTSCamera|GetCameraZoomSpeed)))
  ;[1 1 1] Camera WASD Movement
  (Variables|Default|SetCameraPan (* (Math|Vector|MakeVector (Variables|Default|GetMoveForward_AXIS) (Variables|Default|GetMoveRight_AXIS) 0.0) 2.0))
  ;[1 1 1] Update camera height
  (Variables|Default|SetCameraPan (* (Math|Vector|RotateVector (Variables|Default|GetCameraPan) (Class|KismetMathLibrary|MakeRot 0.0 (.Yaw (Class|KismetMathLibrary|BreakRot (Transformation|GetWorldRotation _mainroot))) 0.0)) (* (Math|Float|SelectFloat (* _cameramovementspeed 2.0) _cameramovementspeed (Game|Player|IsInputKeyDown (Game|GetPlayerController 0) "LeftShift")) (Math|Curves|GetFloatValue (Variables|RTSCamera|GetCameraMoveRateCurve) (Variables|/Script/Engine.SpringArmComponent|GetTargetArmLength (Variables|Default|GetCameraBoom))))))
  (bind _outhit (Collision|LineTraceByChannel (+ (Transformation|GetWorldLocation _mainroot) (Variables|Default|GetCameraPan)) (- (+ (Transformation|GetWorldLocation _mainroot) (Variables|Default|GetCameraPan)) "0, 0,10000.000000") "TraceTypeQuery1" false 0 "None"))
  (Transformation|SetActorLocation (Math|Vector|MakeVector (.X (Math|Vector|BreakVector (+ (.ImpactPoint (Collision|BreakHitResult _outhit)) "0, 0,2000.000000"))) (.Y (Math|Vector|BreakVector (+ (.ImpactPoint (Collision|BreakHitResult _outhit)) "0, 0,2000.000000"))) (Math|Interpolation|FInterpTo (.Z (Math|Vector|BreakVector (Transformation|GetActorLocation))) (.Z (Math|Vector|BreakVector (+ (.ImpactPoint (Collision|BreakHitResult _outhit)) "0, 0,2000.000000"))) DeltaSeconds (Math|Float|SelectFloat 4.0 2.0 (Game|Player|IsInputKeyDown (Game|GetPlayerController 0) "LeftShift")))) false))

(fn ConstructionScript
  (bind _rts_camera (Variables|Default|GetRTS_Camera))
  (Variables|/Script/Engine.SpringArmComponent|SetTargetArmLength (Variables|Default|GetCameraBoom) (Variables|RTSCamera|GetCameraBoomLength))
  (Variables|/Script/Engine.CameraComponent|SetProjectionMode _rts_camera (Variables|RTSCamera|GetProjectionMode))
  (Variables|/Script/Engine.CameraComponent|SetFieldOfView _rts_camera (Variables|RTSCamera|GetFOV))
  (Variables|/Script/Engine.CameraComponent|SetOrthoWidth _rts_camera (Variables|RTSCamera|GetOrthograhicWidth)))