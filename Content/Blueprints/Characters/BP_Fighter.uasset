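; BP_Fighter is a character Blueprint for the Fighter, using a dwarf grunt mesh and the Dwarf_ABP animation Blueprint.
; Its construction script sets the character type, mesh and anim class, reapplies the mesh transform as a noted editor-restart bug workaround, then runs the parent script.
; PlayUniversalAnimation raises a flag for attacks, but plays death directly on the mesh as a non-looping animation.
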(fn ConstructionScript
  (bind _mesh (Variables|Character|GetMesh))
  (Variables|Default|SetCharacterType "NewEnumerator1")
  (Variables|Default|SetCharacterMesh "/Game/Characters/DwarfGrunt/SkelMesh/DwarfGrunt_R_new.DwarfGrunt_R_new")
  ;[1 1 1] Wierd bug requires this to be set every time unreal engine is restarted
  (Transformation|SetRelativeRotation _mesh "0,-90.000000, 0" false)
  (Transformation|SetRelativeLocation _mesh "0, 0,-95.000000" false)
  (Components|SkeletalMesh|SetAnimInstanceClass _mesh "/Game/Characters/DwarfGrunt/Anims/Anim_BP/Dwarf_ABP.Dwarf_ABP_C")
  (|CallParentFunction))

(fn PlayUniversalAnimation
  (params (animation :type UniversalAnimation%20Enum :default "NewEnumerator0"))
  (switch Utilities|FlowControl|Switch|SwitchonUniversalAnimation animation
    (:NewEnumerator0
      (Variables|Default|SetshouldPlayAttackAnim true))
    (:NewEnumerator1
      (Components|Animation|PlayAnimation (Variables|Character|GetMesh) "/Game/Characters/DwarfGrunt/Anims/Death2.Death2" false)))
  (return false))