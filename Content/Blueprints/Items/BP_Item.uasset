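; BP_Item is an item actor that can be picked up and dropped, with a type defaulting to "Generic" and a set of stat bonuses filled at construction.
; Pickup adds normal items to the inventory, then hides and teleports them to a distant void instead of destroying them.
; Container items instead spawn a new Inventory actor for the character and destroy themselves.
; Drop unhides the item and teleports it to the given location.
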(fn ConstructionScript
  (Variables|Default|SetType "Generic")
  (Utilities|Struct|SetmembersinStatBonusSet (Variables|Default|GetBonuses) (Variables|Bonuses|GetStrBonus) (Variables|Bonuses|GetDexBonus) (Variables|Bonuses|GetIntBonus) (Variables|Bonuses|GetWilBonus) (Variables|Bonuses|GetStaBonus)))

(fn Pickup
  (params (Inventory :type Inventory%20Object%20Reference%20%28by%20ref%29) (Character :type BP%20RTS%20Character%20Object%20Reference) (ItemReference :type BP%20Item%20Object%20Reference%20%28by%20ref%29))
  (if (Utilities|Enum|NotEqual(Enum) (Variables|Default|GetType) "Container")
    ;[1 1 1] Normal Item
    (Variables|/Game/Blueprints/Items/Inventory.Inventory_C|SetcurrentItemCount Inventory (+ (Variables|/Game/Blueprints/Items/Inventory.Inventory_C|GetcurrentItemCount Inventory) 1))
    (Utilities|Array|Add (Variables|/Game/Blueprints/Items/Inventory.Inventory_C|GetItems Inventory) ItemReference)
    (Rendering|SetActorHiddenInGame true)
    ;;[1 1 1] Move to void location
    (Transformation|Teleport "0, 0,1000000.000000" "0, 0, 0")
    (else
      ;[1 1 1] Item is an inventory itself
      (bind _returnvalue (Game|SpawnActorfromClass "/Game/Blueprints/Items/Inventory.Inventory_C" (Math|Transform|MakeTransform "0.000000, 0,1000000.000000") true (Game|Player|GetPlayerPawn 0)))
      (Default|AddInventory Character _returnvalue)
      (Actor|DestroyActor))))

(fn Drop
  (params (Location :type Vector))
  (Rendering|SetActorHiddenInGame false)
  (Transformation|Teleport Location "0, 0, 0"))