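; BP_Prop is a damageable environment prop that drops an item when its health runs out.
; Only BP_PhysicalDamage lowers health; at zero or below it spawns ItemDropped at its location and turns off mesh collision, without destroying the actor.
; Its CollisionSphere passes the prop to any overlapping BP_RTS_Character through PropOverlap.
; PlayUniversalAnimation is a stub returning false, and several disconnected leftover nodes never run.
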(event OnComponentBeginOverlap(CollisionSphere)
  (params (OtherActor :type Actor%20Object%20Reference) (OtherComp :type Primitive%20Component%20Object%20Reference) (OtherBodyIndex :type Integer) (bFromSweep :type Boolean) (SweepResult :type Hit%20Result%20Structure%20%28by%20ref%29))
  (bind _asbp_rts_character (Utilities|Casting|CastToBP_RTS_Character OtherActor))
  (Default|PropOverlap _asbp_rts_character self))

(event EventAnyDamage
  (params (Damage :type Float%20%28single-precision%29) (DamageType :type Damage%20Type%20Object%20Reference) (InstigatedBy :type Controller%20Object%20Reference) (DamageCauser :type Actor%20Object%20Reference))
  (bind _returnvalue (Transformation|GetActorLocation))
  (bind (_x _y _z) (Math|Vector|BreakVector _returnvalue))
  (Utilities|Casting|CastToBP_PhysicalDamage DamageType)
  (Variables|Default|SetCurrent%20Health (- (Variables|Default|GetCurrent%20Health) Damage))
  (if (<= (Variables|Default|GetCurrent%20Health) 0.0)
    (Game|SpawnActorfromClass (Variables|Default|GetItem%20Dropped) (Math|Transform|MakeTransform (Math|Vector|MakeVector _x _y (+ _z 0.0))) true 0)
    (Collision|SetCollisionEnabled (Variables|Default|GetMainMesh) "NoCollision")))

(fn ConstructionScript)

(fn PlayUniversalAnimation
  (params (animation :type UniversalAnimation%20Enum))
  (return false))