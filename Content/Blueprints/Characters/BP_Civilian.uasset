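; BP_Civilian is a civilian character Blueprint that configures a parent character class with a dwarf grunt mesh.
; Its construction script sets character type, current and default behavior modes, and mesh before running the parent script.
; Play Universal Animation raises a flag for attacks and plays a non-looping death animation directly on the mesh.
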(fn ConstructionScript
  (Variables|Default|SetCharacterType "NewEnumerator0")
  (Variables|Default|SetBehaviorMode "NewEnumerator3")
  (Variables|Default|SetDefaultBehaviorMode "NewEnumerator3")
  (Variables|Default|SetCharacterMesh "/Game/Characters/DwarfGrunt/SkelMesh/DwarfGrunt_R_new.DwarfGrunt_R_new")
  (|CallParentFunction))

(fn PlayUniversalAnimation
  (params (animation :type UniversalAnimation%20Enum :default "NewEnumerator0"))
  (switch Utilities|FlowControl|Switch|SwitchonUniversalAnimation animation
    (:NewEnumerator0
      (Variables|Default|SetshouldPlayAttackAnim true))
    (:NewEnumerator1
      (Components|Animation|PlayAnimation (Variables|Character|GetMesh) "/Game/Characters/DwarfGrunt/Anims/Death2.Death2" false)))
  (return false))