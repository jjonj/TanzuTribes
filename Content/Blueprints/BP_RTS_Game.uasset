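; RTS game Blueprint that keeps the team registry and answers alliance queries, creating a neutral "None" team at construction.
; CreateTeam appends a team with a sequential Id, default alliance to team 0, and a color derived from the Id through modulo math.
; GetTeam looks teams up by array index.
; AreTeamsAllied checks only the first team's ally list, treating team 0 as allied with everyone.
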(fn ConstructionScript
  ;[1 1 1] Neutral
  (CallFunction|CreateTeam "None"))

(fn CreateTeam
  (params (Name :type Name))
  (bind _returnvalue (Utilities|Array|Add (Variables|Default|GetTeams) (Utilities|Struct|MakeTeam (Variables|Default|GetNextId) (Utilities|Struct|MakeLinearColor (|(x*0.9+0.5)%1.0 (Math|Conversions|ToFloat(Integer) (Variables|Default|GetNextId))) (|(x*0.75+0.5)%1.0 (Math|Conversions|ToFloat(Integer) (Variables|Default|GetNextId))) (|(x*0.4+0.5)%1.0 (Math|Conversions|ToFloat(Integer) (Variables|Default|GetNextId))) 0.0) (Utilities|Array|MakeArray 0) Name)))
  (Variables|Default|SetNextId (+ _returnvalue 1))
  (return (Utilities|Struct|MakeTeam (Variables|Default|GetNextId) (Utilities|Struct|MakeLinearColor (|(x*0.9+0.5)%1.0 (Math|Conversions|ToFloat(Integer) (Variables|Default|GetNextId))) (|(x*0.75+0.5)%1.0 (Math|Conversions|ToFloat(Integer) (Variables|Default|GetNextId))) (|(x*0.4+0.5)%1.0 (Math|Conversions|ToFloat(Integer) (Variables|Default|GetNextId))) 0.0) (Utilities|Array|MakeArray 0) Name)))

(fn GetTeam
  (params (id :type Integer))
  (return (Utilities|Array|Get(acopy) (Variables|Default|GetTeams) id)))

(fn AreTeamsAllied
  (params (team%201%20id :type Integer) (team%202%20id :type Integer))
  (bind _team (CallFunction|GetTeam team%201%20id))
  (return (Math|Boolean|ORBoolean (!= (Utilities|Array|FindItem (.alliedTeamIds (Utilities|Struct|BreakTeam _team)) team%202%20id) -1) (== team%201%20id 0) (== team%202%20id 0))))