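; Experimental construction manager that turns queued build configs into finished buildings by way of temporary proxy actors.
; QueueConstruction spawns a proxy at the config transform, binds its completion event, stores both in parallel arrays, then initializes it with work hours and hardcoded workers.
; On completion, FinishConstruction finds the config by the proxy's index, destroys the proxy, removes both entries and spawns the building class at the same transform.
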(event Custom|OnConstructionCompleted
  (params (Proxy :type BP%20Construction%20Proxy%20Object%20Reference))
  (CallFunction|FinishConstruction Proxy))

(fn ConstructionScript)

(fn QueueConstruction
  (params (Config :type STRUCT%20Construction%20Conf%20Structure))
  (bind (_buildingclass _proxyclass _transform _workhoursneeded) (Utilities|Struct|BreakSTRUCT_ConstructionConf Config))
  (bind _returnvalue (Game|SpawnActorfromClass _proxyclass _transform false))
  (bind _asbp_constructionproxy_c (Utilities|Casting|CastToBP_ConstructionProxy _returnvalue))
  (EventDispatchers|BindEventtoConstructionCompleted _asbp_constructionproxy_c (EventDispatchers|CreateEvent self :!event Custom|OnConstructionCompleted))
  (Utilities|Array|Add (Variables|Default|GetProxies) _asbp_constructionproxy_c)
  (Utilities|Array|Add (Variables|Default|GetQueue) Config)
  (Default|Initialize _asbp_constructionproxy_c _workhoursneeded 0.0)
  (Default|SetWorkers _asbp_constructionproxy_c (Utilities|Array|MakeArray 1 2)))

(fn FinishConstruction
  (params (Proxy :type BP%20Construction%20Proxy%20Object%20Reference))
  (LocalVariables|SetIndex (Utilities|Array|FindItem (Variables|Default|GetProxies) Proxy))
  (LocalVariables|SetConfig (Utilities|Array|Get(acopy) (Variables|Default|GetQueue) (LocalVariables|GetIndex)))
  (Actor|DestroyActor Proxy)
  (Utilities|Array|RemoveIndex (Variables|Default|GetQueue) (LocalVariables|GetIndex))
  (Utilities|Array|RemoveIndex (Variables|Default|GetProxies) (LocalVariables|GetIndex))
  (Game|SpawnActorfromClass (.BuildingClass (Utilities|Struct|BreakSTRUCT_ConstructionConf (LocalVariables|GetConfig))) (.Transform (Utilities|Struct|BreakSTRUCT_ConstructionConf (LocalVariables|GetConfig))) false))